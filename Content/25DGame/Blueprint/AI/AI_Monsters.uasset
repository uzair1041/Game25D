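; AI controller for monster characters that steers each possessed monster toward the player.
; On possess it caches the pawn as a BPC_MasterMonster, and on begin play it caches the first player's pawn.
; Every tick it takes the look-at rotation from monster to player and passes its forward vector to the monster's FollowPlayer function.
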(event EventBeginPlay
  (Variables|Default|SetPlayer (Game|Player|GetPlayerPawn 0)))

(event EventTick
  (params (DeltaSeconds :type Float%20%28single-precision%29))
  (Default|FollowPlayer (Variables|Default|GetPossessed%20Pawn) (Math|Vector|GetForwardVector (Math|Rotator|FindLookatRotation (Transformation|GetActorLocation (Variables|Default|GetPossessed%20Pawn)) (Transformation|GetActorLocation (Variables|Default|GetPlayer))))))

(event EventPossess
  (params (PossessedPawn :type Pawn%20Object%20Reference))
  (bind _asbpc_master_monster (Utilities|Casting|CastToBPC_MasterMonster PossessedPawn))
  (Variables|Default|SetPossessed%20Pawn _asbpc_master_monster))

(fn ConstructionScript)