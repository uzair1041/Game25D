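; AC_Health is a health component that tracks a current health value for the actor it belongs to.
; BeginPlay sets current health to the maximum, and DamageHealth subtracts damage with a floor at zero and prints the result.
; DamageHealth then sets IsAlive to true when health is at or below zero, so the flag reads opposite to its name.
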(event EventBeginPlay
  (Variables|Default|SetCurrentHealth (Variables|Default|GetMaxHealth)))

(event EventTick
  (params (DeltaSeconds :type Float%20%28single-precision%29)))

(fn DamageHealth
  (params (DamageTaken :type Float%20%28double-precision%29))
  (Variables|Default|SetCurrentHealth (Math|Float|Max(Float) (- (Variables|Default|GetCurrentHealth) DamageTaken) 0.0))
  (Development|PrintString (Utilities|String|ToString(Float) (Variables|Default|GetCurrentHealth)))
  (Variables|Default|SetIsAlive (<= (Variables|Default|GetCurrentHealth) 0.0)))