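; Player hero character for a 2.5D game, handling Enhanced Input movement and a melee attack.
; IA_Movement drives world X/Y movement, and IA_Attack plays an override animation that holds IsAttacking until completed or cancelled.
; Both inputs are gated by CanMove, which requires ACHealth.IsAlive and IsAttacking to both be false.
; AttackHitBox damages overlapping BPC_MasterMonster actors; its caller is outside these graphs.
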(event Input|EnhancedActionEvents|EnhancedInputActionIA_Movement
  (params (ActionValue :type Vector%202D%20Structure) (ElapsedSeconds :type Float%20%28double-precision%29) (TriggeredSeconds :type Float%20%28double-precision%29) (InputAction :type Input%20Action%20Object%20Reference :default "/Game/25DGame/Blueprint/Gameplay/Input/IA_Movement.IA_Movement"))
  (bind (_x _y) (Math|Vector2D|BreakVector2D ActionValue))
  (if (CallFunction|CanMove)
    (Pawn|Input|AddMovementInput "1.000000,0.000000,0.000000" _x false)
    (Pawn|Input|AddMovementInput "0.000000,1.000000,0.000000" _y false)))

(event Input|EnhancedActionEvents|EnhancedInputActionIA_Attack
  (params (ActionValue :type Boolean) (ElapsedSeconds :type Float%20%28double-precision%29) (TriggeredSeconds :type Float%20%28double-precision%29) (InputAction :type Input%20Action%20Object%20Reference :default "/Game/25DGame/Blueprint/Gameplay/Input/IA_Attack.IA_Attack"))
  (:Started
    (if (CallFunction|CanMove)
      (|PlayAnimationOverridewithCallbacks (Variables|/Script/PaperZD.PaperZDAnimationComponent|GetAnimInstance (Variables|Default|GetAnimationComponent)) "/Game/25DGame/Blueprint/Characters/PlayerHero/AnimSequences/Attack.Attack" "DefaultSlot" 1.0 0.0
        (:then
          (Variables|Default|SetIsAttacking true))
        (:OnCompleted
          (Variables|Default|SetIsAttacking false :!label _label))
        (:OnCancelled
          (goto _label))))))

(event EventBeginPlay
  (|CallParentFunction)
  (Input|AddMappingContext (PlayerController|LocalPlayerSubsystems|GetEnhancedInputLocalPlayerSubsystem (Game|GetPlayerController 0)) "/Game/25DGame/Blueprint/Gameplay/Input/IMC_25D.IMC_25D" 0 "(bIgnoreAllPressedKeysUntilRelease=True,bForceImmediately=False,bNotifyUserSettings=False)"))

(event Collision|EventActorBeginOverlap
  (params (OtherActor :type Actor%20Object%20Reference))
  (|CallParentFunction OtherActor) ; This node is disabled and will not be called.\nDrag off pins to build functionality.
)

(event EventTick
  (params (DeltaSeconds :type Float%20%28single-precision%29))
  (|CallParentFunction DeltaSeconds) ; This node is disabled and will not be called.\nDrag off pins to build functionality.
)

(fn ConstructionScript
  (|CallParentFunction))

(fn AttackHitBox
  (bind _arrayelement (Utilities|Array|ReverseforEachLoop (Collision|GetOverlappingActors (Variables|Default|GetHitBox) "/Game/25DGame/Blueprint/Characters/BPC_MasterMonster.BPC_MasterMonster_C" :!class /Script/Engine.PrimitiveComponent))
    (:LoopBody
      (Game|Damage|ApplyDamage _arrayelement 1.0 0 0))))

(fn CanMove
  (return (and (not (Variables|/Game/25DGame/Blueprint/Component/AC_Health.AC_Health_C|GetIsAlive (Variables|Default|GetAC_Health))) (not (Variables|Default|GetIsAttacking)))))