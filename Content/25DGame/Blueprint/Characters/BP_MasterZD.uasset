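; BP_MasterZD is a PaperZD character base Blueprint that handles damage response and death for 2.5D characters.
; AnyDamage checks ACHealth's IsAlive flag, which reads inverted: damage applies when false, and death follows when it turns true.
; Damage triggers a brief red sprite flash through a retriggerable delay.
; Death jumps the animation instance to its Death node, then destroys the actor only if it casts to BPC_MasterMonster.
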(event Custom|SpriteHit
  (Sprite|SetSpriteColor (Variables|Default|GetSprite) "(R=1.000000,G=0.000000,B=0.000000,A=1.000000)")
  (Utilities|FlowControl|RetriggerableDelay 0.2)
  (Sprite|SetSpriteColor (Variables|Default|GetSprite) "(R=1.000000,G=1.000000,B=1.000000,A=1.000000)"))

(event EventBeginPlay)

(event Collision|EventActorBeginOverlap
  (params (OtherActor :type Actor%20Object%20Reference)))

(event EventTick
  (params (DeltaSeconds :type Float%20%28single-precision%29)))

(event Game|Damage|EventAnyDamage
  (params (Damage :type Float%20%28single-precision%29) (DamageType :type Damage%20Type%20Object%20Reference) (InstigatedBy :type Controller%20Object%20Reference) (DamageCauser :type Actor%20Object%20Reference))
  (if (not (Variables|/Game/25DGame/Blueprint/Component/AC_Health.AC_Health_C|GetIsAlive (Variables|Default|GetAC_Health)))
    (Default|DamageHealth (Variables|Default|GetAC_Health) Damage)
    (CallFunction|SpriteHit)
    (if (Variables|/Game/25DGame/Blueprint/Component/AC_Health.AC_Health_C|GetIsAlive (Variables|Default|GetAC_Health))
      (Class|PaperZDAnimInstance|JumptoNode (Variables|/Script/PaperZD.PaperZDAnimationComponent|GetAnimInstance (Variables|Default|GetAnimationComponent)) "Death" "None")
      (Utilities|Casting|CastToBPC_MasterMonster self)
      (Actor|DestroyActor))))

(fn ConstructionScript)