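; BPC_MasterMonster is a monster character, named as the master class, that moves on request and damages the player hero on contact.
; FollowPlayer adds movement input along a supplied world direction, but only when the ACHealth IsAlive flag is false.
; A HitBox overlap with the hero's DamageBox applies damage to the hero.
; BeginPlay, ActorBeginOverlap and Tick are disabled placeholders.
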(event OnComponentBeginOverlap(HitBox)
  (params (OverlappedComponent :type Primitive%20Component%20Object%20Reference) (OtherActor :type Actor%20Object%20Reference) (OtherComp :type Primitive%20Component%20Object%20Reference) (OtherBodyIndex :type Integer) (bFromSweep :type Boolean) (SweepResult :type Hit%20Result%20Structure%20%28by%20ref%29))
  (bind _asbpc_player_hero (Utilities|Casting|CastToBPC_PlayerHero OtherActor))
  (if (== (Variables|/Game/25DGame/Blueprint/Characters/BP_MasterZD.BP_MasterZD_C|GetDamageBox _asbpc_player_hero) OtherComp)
    (Game|Damage|ApplyDamage _asbpc_player_hero 1.0 0 0)))

(event Custom|FollowPlayer
  (params (WorldDirection :type Vector))
  (if (not (Variables|/Game/25DGame/Blueprint/Component/AC_Health.AC_Health_C|GetIsAlive (Variables|Default|GetAC_Health)))
    (Pawn|Input|AddMovementInput WorldDirection 1.0 false)))

(event EventBeginPlay
  (|CallParentFunction) ; This node is disabled and will not be called.\nDrag off pins to build functionality.
)

(event Collision|EventActorBeginOverlap
  (params (OtherActor :type Actor%20Object%20Reference))
  (|CallParentFunction OtherActor) ; This node is disabled and will not be called.\nDrag off pins to build functionality.
)

(event EventTick
  (params (DeltaSeconds :type Float%20%28single-precision%29))
  (|CallParentFunction DeltaSeconds) ; This node is disabled and will not be called.\nDrag off pins to build functionality.
)

(fn ConstructionScript
  (|CallParentFunction))